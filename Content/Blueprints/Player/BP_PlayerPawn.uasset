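; Player pawn for a tower defense game, handling camera movement, tower building and selection, gold, and wave start.
; Number keys buy towers from a data table, charging gold immediately; the held tower follows cursor traces until clicked onto a free plot.
; GameSubsystem events drive upgrade, sell and move requests and broadcast gold changes.
; Sell refunds and move fees use accumulated tier costs, halved once the tower has dealt damage.
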(event `self.ReceiveBeginPlay`
  (add `GameSubsystem.OnTowerUpgradeRequest` (subsystem `GameSubsystem`) (`|CreateDelegate` :!event `OnTowerUpgradeRequestEvent`))
  (add `GameSubsystem.OnTowerSellRequest` (subsystem `GameSubsystem`) (`|CreateDelegate` :!event `OnTowerSellRequestEvent`))
  (add `GameSubsystem.OnTowerMoveRequest` (subsystem `GameSubsystem`) (`|CreateDelegate` :!event `OnTowerMoveRequestEvent`)))

(event `EnhancedInput|/Game/Input/Actions/IA_Move`
  (params (ActionValue :type "Vector2D Structure") (ElapsedSeconds :type "Float (double-precision)") (TriggeredSeconds :type "Float (double-precision)") (InputAction :type "InputAction Object Reference" :default "/Game/Input/Actions/IA_Move.IA_Move"))
  (bind (_x _y) (`KismetMathLibrary.BreakVector2D` ActionValue))
  (:`Triggered`
    (`self.AddMovementInput` (`self.GetActorForwardVector`) _x)
    (`self.AddMovementInput` (`self.GetActorRightVector`) _y)))

(event `EnhancedInput|/Game/Input/Actions/IA_Zoom`
  (params (ActionValue :type "Float (double-precision)") (ElapsedSeconds :type "Float (double-precision)") (TriggeredSeconds :type "Float (double-precision)") (InputAction :type "InputAction Object Reference" :default "/Game/Input/Actions/IA_Zoom.IA_Zoom"))
  (bind _springarm (`self.SpringArm`))
  (:`Triggered`
    (set `SpringArmComponent.TargetArmLength` (`KismetMathLibrary.FClamp` (- (`SpringArmComponent.TargetArmLength` _springarm) (* ActionValue 100.0)) 200.0 2000.0) _springarm)))

(event `EnhancedInput|/Game/Input/Actions/IA_Rotate`
  (params (ActionValue :type "Float (double-precision)") (ElapsedSeconds :type "Float (double-precision)") (TriggeredSeconds :type "Float (double-precision)") (InputAction :type "InputAction Object Reference" :default "/Game/Input/Actions/IA_Rotate.IA_Rotate"))
  (:`Triggered`
    (`self.K2_AddActorWorldRotation` (`KismetMathLibrary.MakeRotator` 0.0 0.0 ActionValue))))

(event `EnhancedInput|/Game/Input/Actions/IA_Click`
  (params (ActionValue :type Boolean) (ElapsedSeconds :type "Float (double-precision)") (TriggeredSeconds :type "Float (double-precision)") (InputAction :type "InputAction Object Reference" :default "/Game/Input/Actions/IA_Click.IA_Click"))
  (:`Triggered`
    (`/Engine/EditorBlueprintResources/StandardMacros.IsValid` (`self.HeldTower`)
      (:`Is Valid`
        (bind (_bsuccess _bistowerplot _outlocation _outplot _outprimitive) (`self.TraceForTowerPlot`))
        (if (and _bsuccess _bistowerplot)
          (`self.K2_SetActorLocation` (`self.HeldTower`) _outlocation false false)
          (`/Game/Blueprints/Tower/BP_TowerPlot.SlotUpdate` _outplot _outprimitive true)
          (message `/Game/Blueprints/Interfaces/BPI_Tower.OnTowerPlaced` (`self.HeldTower`))
          (set `self.HeldTower` null)))
      (:`Is Not Valid`
        (bind (_bsuccess_2 _outlocation_2 _outhitactor) (`self.TraceFromScreen`))
        (if _bsuccess_2
          (bind _asbp_tower_base (cast `/Game/Blueprints/Tower/BP_TowerBase` _outhitactor)
            (:`then`
              (`self.HandleSelectTower` _asbp_tower_base))
            (:`CastFailed`
              (`self.HandleDeselectTower`))))))))

(event `self.ReceiveTick`
  (params (DeltaSeconds :type "Float (single-precision)"))
  (`/Engine/EditorBlueprintResources/StandardMacros.IsValid` (`self.HeldTower`)
    (:`Is Valid`
      (bind (_bsuccess _bistowerplot _outlocation) (`self.TraceForTowerPlot`))
      (if _bsuccess
        (`self.K2_SetActorLocation` (`self.HeldTower`) _outlocation false false)
        (if _bistowerplot
          _)))))

(event `Key|One`
  (params (Key :type "Key Structure"))
  ;[1 0 0] REFACTOR ASAP
  (:`Pressed`
    (bind (_bsuccess _outtowerclass _outtowerdata _outrowhandle _outmaxtowerupgradeindex) (`self.GetTowerData` "Ballista"))
    (if _bsuccess
      (`/Engine/EditorBlueprintResources/StandardMacros.IsValid` (`self.HeldTower`)
        (:`Is Valid`
          (message `/Game/Blueprints/Interfaces/BPI_Tower.OnDeleteTower` (`self.HeldTower`)))
        (:`Is Not Valid`
          _))
      (`self.SpawnTower` _outtowerclass _outtowerdata _outrowhandle _outmaxtowerupgradeindex))))

(event `Key|Two`
  (params (Key :type "Key Structure"))
  ;[1 0 0] REFACTOR ASAP
  (:`Pressed`
    (bind (_bsuccess _outtowerclass _outtowerdata _outrowhandle _outmaxtowerupgradeindex) (`self.GetTowerData` "Cannon"))
    (if _bsuccess
      (`/Engine/EditorBlueprintResources/StandardMacros.IsValid` (`self.HeldTower`)
        (:`Is Valid`
          (message `/Game/Blueprints/Interfaces/BPI_Tower.OnDeleteTower` (`self.HeldTower`)))
        (:`Is Not Valid`
          _))
      (`self.SpawnTower` _outtowerclass _outtowerdata _outrowhandle _outmaxtowerupgradeindex))))

(event `Key|Three`
  (params (Key :type "Key Structure"))
  ;[1 0 0] REFACTOR ASAP
  (:`Pressed`
    (bind (_bsuccess _outtowerclass _outtowerdata _outrowhandle _outmaxtowerupgradeindex) (`self.GetTowerData` "Catapult"))
    (if _bsuccess
      (`/Engine/EditorBlueprintResources/StandardMacros.IsValid` (`self.HeldTower`)
        (:`Is Valid`
          (message `/Game/Blueprints/Interfaces/BPI_Tower.OnDeleteTower` (`self.HeldTower`)))
        (:`Is Not Valid`
          _))
      (`self.SpawnTower` _outtowerclass _outtowerdata _outrowhandle _outmaxtowerupgradeindex))))

(event `Key|Four`
  (params (Key :type "Key Structure"))
  ;[1 0 0] REFACTOR ASAP
  (:`Pressed`
    (bind (_bsuccess _outtowerclass _outtowerdata _outrowhandle _outmaxtowerupgradeindex) (`self.GetTowerData` "Buff"))
    (if _bsuccess
      (`/Engine/EditorBlueprintResources/StandardMacros.IsValid` (`self.HeldTower`)
        (:`Is Valid`
          (message `/Game/Blueprints/Interfaces/BPI_Tower.OnDeleteTower` (`self.HeldTower`)))
        (:`Is Not Valid`
          _))
      (`self.SpawnTower` _outtowerclass _outtowerdata _outrowhandle _outmaxtowerupgradeindex))))

(event `Key|SpaceBar`
  (params (Key :type "Key Structure"))
  (:`Pressed`
    (`GameSubsystem.OnPlayerStartWave` (subsystem `GameSubsystem`))))

(event `OnTowerUpgradeRequestEvent`
  (params (InTowerBase :type "TowerBase Object Reference"))
  (bind (_towerrowhandle_datatable _towerrowhandle_rowname) (break `DataTableRowHandle` (`TowerBase.TowerRowHandle` InTowerBase)))
  (bind _returnvalue (+ (`TowerBase.TowerUpgradeIndex` InTowerBase) 1))
  (bind _returnvalue_2 (`|GetDataTableRow` _towerrowhandle_datatable _towerrowhandle_rowname)
    (:`then`
      (bind (_towername _towertype _towerdata) (break `TowerCollection` _returnvalue_2))
      (if (not (> _returnvalue (`KismetArrayLibrary.Array_LastIndex` _towerdata)))
        (bind _output (`|GetArrayItem` _towerdata _returnvalue))
        (bind _cost (break `TowerData` _output))
        (if (>= (`self.Gold`) _cost)
          (`self.OnBuyTowerEvent` _cost)
          (message `/Game/Blueprints/Interfaces/BPI_Tower.OnTowerUpgrade` InTowerBase _output _returnvalue))))))

(event `OnTowerSellRequestEvent`
  (params (InTowerBase :type "TowerBase Object Reference"))
  (bind (_bsuccess _outcost) (`self.GetTowerCost` InTowerBase 0.5))
  (if _bsuccess
    (message `/Game/Blueprints/Interfaces/BPI_Tower.OnDeleteTower` InTowerBase)
    (`self.OnMoneyReward` _outcost)))

(event `OnTowerMoveRequestEvent`
  (params (InTowerBase :type "TowerBase Object Reference"))
  (bind (_bsuccess _outcost) (`self.GetTowerCost` InTowerBase 0.5))
  (if (and _bsuccess (>= (`self.Gold`) _outcost))
    (`self.OnBuyTowerEvent` _outcost)
    (message `/Game/Blueprints/Interfaces/BPI_Tower.OnMoveTower` InTowerBase)
    (set `self.HeldTower` InTowerBase)))

(event `/Game/Blueprints/Interfaces/BPI_Player.OnMoneyReward`
  (params (InReward :type Integer))
  (bind _output_get (set `self.Gold` (+ InReward (`self.Gold`))))
  (`GameSubsystem.OnGoldUpdated` (subsystem `GameSubsystem`) _output_get))

(event `OnBuyTowerEvent`
  (params (InCost :type Integer))
  (bind _output_get (set `self.Gold` (- (`self.Gold`) InCost)))
  (`GameSubsystem.OnGoldUpdated` (subsystem `GameSubsystem`) _output_get))

(fn `GetTowerCost`
  (params (InTowerBase :type "TowerBase Object Reference") (InMultiplier :type "Float (double-precision)"))
  (returns (bSuccess :type Boolean) (OutCost :type Integer))
  (locals (AccumulatedCost :type Integer))
  (bind (_towerrowhandle_datatable _towerrowhandle_rowname) (break `DataTableRowHandle` (`TowerBase.TowerRowHandle` InTowerBase)))
  (bind _returnvalue (`|GetDataTableRow` _towerrowhandle_datatable _towerrowhandle_rowname)
    (:`then`
      (for _index (range (+ (`TowerBase.TowerUpgradeIndex` InTowerBase) 1))
        (set `local.AccumulatedCost` (+ (`.Cost` (break `TowerData` (`|GetArrayItem` (`.TowerData` (break `TowerCollection` _returnvalue)) _index))) (`local.AccumulatedCost`))))
      (if (> (`.DamageDealt` (break `TowerStats` (`TowerBase.TowerStats` (`local.InTowerBase`)))) 0.0)
        (return true (/ (`local.AccumulatedCost`) 2))
        (else
          (return true (`local.AccumulatedCost`)))))
    (:`RowNotFound`
      (return false 0))))

(fn `GetTowerData`
  (params (InTowerName :type Name))
  (returns (bSuccess :type Boolean) (OutTowerClass :type "TowerBase Class Reference") (OutTowerData :type "TowerData Structure (by ref)") (OutRowHandle :type "DataTableRowHandle Structure") (OutMaxTowerUpgradeIndex :type Integer))
  (bind _returnvalue (`|GetDataTableRow` (`self.TowerCollection`) InTowerName)
    (:`then`
      (bind (_towername _towertype _towerdata) (break `TowerCollection` _returnvalue))
      (if (> (`KismetArrayLibrary.Array_Length` _towerdata) 0)
        (bind _output (`|GetArrayItem` _towerdata))
        (bind _cost (break `TowerData` _output))
        (if (>= (`self.Gold`) _cost)
          (`self.OnBuyTowerEvent` _cost)
          (return true _towertype _output (make `DataTableRowHandle` (`self.TowerCollection`) (`local.InTowerName`)) (`KismetArrayLibrary.Array_LastIndex` _towerdata))
          (else
            (return false null (struct) (struct) 0)))
        (else
          (return false null (struct) (struct) 0))))
    (:`RowNotFound`
      (return false null (struct) (struct) 0))))

(fn `HandleDeselectTower`
  (`/Engine/EditorBlueprintResources/StandardMacros.IsValid` (`self.ClickedTowerRef`)
    (:`Is Valid`
      (`/Game/Blueprints/Tower/BP_TowerBase.OnDeselectTowerEvent` (`self.ClickedTowerRef`))
      (`TowerSubsystem.OnTowerDeselected` (subsystem `TowerSubsystem`)))))

(fn `HandleSelectTower`
  (params (ClickedTowerRef :type "/Game/Blueprints/Tower/BP_TowerBase Object Reference"))
  (`/Engine/EditorBlueprintResources/StandardMacros.IsValid` (`self.ClickedTowerRef`)
    (:`Is Valid`
      (`/Game/Blueprints/Tower/BP_TowerBase.OnDeselectTowerEvent` (`self.ClickedTowerRef`)))
    (:`Is Not Valid`
      _))
  (bind _output_get (set `self.ClickedTowerRef` ClickedTowerRef))
  (`/Game/Blueprints/Tower/BP_TowerBase.OnSelectTowerEvent` _output_get))

(fn `SpawnTower`
  (params (InputPin :type "TowerBase Class Reference") (TowerData :type "TowerData Structure") (InRowHandle :type "DataTableRowHandle Structure") (InMaxTowerUpgradeIndex :type Integer))
  (bind _returnvalue (`|SpawnActorFromClass` InputPin (`KismetMathLibrary.MakeTransform` (0.0 0.0 0.0)) "Undefined" "MultiplyWithRoot" null TowerData InRowHandle InMaxTowerUpgradeIndex null))
  (bind _output_get (set `self.HeldTower` _returnvalue))
  (bind _asbp_tower_base (cast `/Game/Blueprints/Tower/BP_TowerBase` _output_get))
  (`self.HandleSelectTower` _asbp_tower_base))

(fn `TraceForTowerPlot`
  (returns (bSuccess :type Boolean) (bIsTowerPlot :type Boolean) (OutLocation :type "Vector Structure") (OutPlot :type "/Game/Blueprints/Tower/BP_TowerPlot Object Reference") (OutPrimitive :type "PrimitiveComponent Object Reference"))
  (bind (_worldlocation _worlddirection) (`PlayerController.DeprojectMousePositionToWorld` (`GameplayStatics.GetPlayerController` 0)))
  (bind (_outhit _returnvalue) (`KismetSystemLibrary.LineTraceSingleForObjects` _worldlocation (+ _worldlocation (* _worlddirection 5000.0)) (`|MakeArray` "ObjectTypeQuery9" "ObjectTypeQuery1" :!type "EObjectTypeQuery Enum")))
  (if _returnvalue
    (bind (_bblockinghit _binitialoverlap _time _distance _location _impactpoint _normal _impactnormal _physmat _hitactor _hitcomponent) (`GameplayStatics.BreakHitResult` _outhit))
    (bind _asbp_tower_plot (cast `/Game/Blueprints/Tower/BP_TowerPlot` _hitactor)
      (:`then`
        (bind (_value _returnvalue_2) (`BlueprintMapLibrary.Map_Find` (`/Game/Blueprints/Tower/BP_TowerPlot.BoxMap` _asbp_tower_plot) _hitcomponent))
        (if (and (not _value) _returnvalue_2)
          (return true true (`SceneComponent.K2_GetComponentLocation` _hitcomponent) _asbp_tower_plot _hitcomponent)
          (else
            (return true false _location null null))))
      (:`CastFailed`
        (return true false _location null null)))
    (else
      (return false false (0.0 0.0 0.0) null null))))

(fn `TraceFromScreen`
  (returns (bSuccess :type Boolean) (OutLocation :type "Vector Structure") (OutHitActor :type "Actor Object Reference"))
  (bind (_worldlocation _worlddirection) (`PlayerController.DeprojectMousePositionToWorld` (`GameplayStatics.GetPlayerController` 0)))
  (bind (_outhit _returnvalue) (`KismetSystemLibrary.LineTraceSingle` _worldlocation (+ _worldlocation (* _worlddirection 5000.0)) "TraceTypeQuery1"))
  (if _returnvalue
    (bind (_bblockinghit _binitialoverlap _time _distance _location _impactpoint _normal _impactnormal _physmat _hitactor) (`GameplayStatics.BreakHitResult` _outhit))
    (return true _location _hitactor)
    (else
      (return false (0.0 0.0 0.0) null))))

(fn `UserConstructionScript`)