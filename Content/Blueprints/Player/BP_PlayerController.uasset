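; Player controller that tracks the player's lives and ends the game when too many enemies reach the end.
; On BeginPlay it creates the HUD, adds the default Enhanced Input mapping context, shows the mouse cursor and binds to the enemy-reach-end event.
; Each such event decrements Lives and updates the HUD; at zero or below it shows the loss state and pauses the game.
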(event `self.ReceiveBeginPlay`
  (bind _returnvalue (`|CreateWidget` "/Game/Widget/WBP_HUD.WBP_HUD_C"))
  (bind _output_get (set `self.WBP_HUDRef` _returnvalue))
  (`UserWidget.AddToViewport` _output_get 0)
  (`/Game/Widget/WBP_HUD.SetLivesLeft` (`self.WBP_HUDRef`) (`self.Lives`))
  (`EnhancedInputSubsystemInterface.AddMappingContext` (subsystem `EnhancedInputLocalPlayerSubsystem`) "/Game/Input/IMC_Default.IMC_Default" 0 (struct))
  (set `self.bShowMouseCursor` true)
  (add `self.EnemyReachEnd` (`|CreateDelegate` :!event `EnemyReachEndEvent`)))

(event `EnemyReachEndEvent`
  (`/Engine/EditorBlueprintResources/StandardMacros.DecrementInt` (`self.Lives`)
    (:`  `
      (`/Game/Widget/WBP_HUD.SetLivesLeft` (`self.WBP_HUDRef`) (`self.Lives`))
      (if (<= (`self.Lives`) 0)
        (`/Game/Widget/WBP_HUD.GameIsLost` (`self.WBP_HUDRef`))
        (`GameplayStatics.SetGamePaused` true)))))

(fn `UserConstructionScript`)