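; Base tower for a tower-defense game that automatically fires arcing projectiles at enemies in range.
; A range sphere maintains the target list; Tick aims the weapon at the first entry and fires on cooldown.
; A projectile waits attached to the weapon, launches with a suggested arc velocity, and is replaced after half the cooldown.
; It also handles selection decal, kill/damage stats, upgrades, and freeing its plot via downward trace when moved or deleted.
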(event `self.ReceiveBeginPlay`
  (bind ((`Range` _range)) (break `TowerData` (`self.TowerData`)))
  (set `self.CooldownTimer` (`.Cooldown` (break `TowerData` (`self.TowerData`))))
  (`self.SpawnNewProjectile`)
  (`SphereComponent.SetSphereRadius` (`self.SphereRadius`) _range false)
  (`SceneComponent.SetWorldScale3D` (`self.Decal`) (`KismetMathLibrary.Conv_DoubleToVector` (/ _range 100.0)))
  (`SceneComponent.SetHiddenInGame` (`self.Decal`) true false))

(event `self.ReceiveTick`
  (params (DeltaSeconds :type "Float (single-precision)"))
  (bind _targets (`self.Targets`))
  (bind (_returnvalue_roll _returnvalue_pitch _returnvalue_yaw) (`KismetMathLibrary.BreakRotator` (`SceneComponent.K2_GetComponentRotation` (`self.WeaponPropMesh`))))
  (bind (_returnvalue_roll_2 _returnvalue_pitch_2 _returnvalue_yaw_2) (`KismetMathLibrary.BreakRotator` (`KismetMathLibrary.FindLookAtRotation` (`SceneComponent.K2_GetComponentLocation` (`self.WeaponBaseMesh`)) (`self.K2_GetActorLocation` (`|GetArrayItem` _targets)))))
  (if (`self.bTowerActive`)
    (set `self.CooldownTimer` (+ DeltaSeconds (`self.CooldownTimer`)))
    (if (`KismetArrayLibrary.Array_IsNotEmpty` _targets)
      (`SceneComponent.K2_SetWorldRotation` (`self.WeaponBaseMesh`) (`KismetMathLibrary.MakeRotator` 0.0 0.0 _returnvalue_yaw_2) false false)
      (if (`self.bShouldTowerPitch`)
        (`SceneComponent.K2_SetWorldRotation` (`self.WeaponPropMesh`) (`KismetMathLibrary.MakeRotator` 0.0 _returnvalue_pitch_2 _returnvalue_yaw) false false))
      (if (> (`self.CooldownTimer`) (`.Cooldown` (break `TowerData` (`self.TowerData`))))
        (set `self.CooldownTimer` 0.0)
        (bind (_bsuccess _asbp_enemy_base) (`self.FindNextValidTarget`))
        (if _bsuccess
          (set `self.CurrentTarget` _asbp_enemy_base)
          (`self.Fire`))))))

(event `Fire`
  (`/Engine/EditorBlueprintResources/StandardMacros.IsValid` (`self.SpawnedProjectile`)
    (:`Is Valid`
      (`self.K2_DetachFromActor` (`self.SpawnedProjectile`) "KeepWorld" "KeepWorld" "KeepWorld")
      (bind _outlaunchvelocity (`GameplayStatics.SuggestProjectileVelocity_CustomArc` (`self.K2_GetActorLocation` (`self.SpawnedProjectile`)) (`self.K2_GetActorLocation` (`self.CurrentTarget`))))
      (`/Game/Blueprints/Tower/Projectiles/BP_ProjectileBase.Fire` (`self.SpawnedProjectile`) _outlaunchvelocity (`self.CurrentTarget`))
      (set `self.SpawnedProjectile` null)
      (`self.QueNewProjectile`))))

(event `OnSelectTowerEvent`
  (`SceneComponent.SetHiddenInGame` (`self.Decal`) false false)
  (add `self.UpdateStats` (`|CreateDelegate` :!event `OnUpdateStatsEvent`))
  (`TowerSubsystem.OnTowerSelected` (subsystem `TowerSubsystem`) self))

(event `OnDeselectTowerEvent`
  (`SceneComponent.SetHiddenInGame` (`self.Decal`) true false)
  (remove `self.UpdateStats` (`|CreateDelegate` :!event `OnUpdateStatsEvent`)))

(event `OnUpdateStatsEvent`
  (`TowerSubsystem.OnTowerSelected` (subsystem `TowerSubsystem`) self))

(event `QueNewProjectile`
  (`KismetSystemLibrary.Delay` (/ (`.Cooldown` (break `TowerData` (`self.TowerData`))) 2.0))
  (`self.SpawnNewProjectile`))

(event `self.SphereRadius.OnComponentBeginOverlap`
  (params (OverlappedComponent :type "PrimitiveComponent Object Reference") (OtherActor :type "Actor Object Reference") (OtherComp :type "PrimitiveComponent Object Reference") (OtherBodyIndex :type Integer) (bFromSweep :type Boolean) (SweepResult :type "HitResult Structure (by ref)"))
  (if (not (`KismetArrayLibrary.Array_Contains` (`self.Targets`) OtherActor))
    (`KismetArrayLibrary.Array_Add` (`self.Targets`) OtherActor)))

(event `self.SphereRadius.OnComponentEndOverlap`
  (params (OverlappedComponent :type "PrimitiveComponent Object Reference") (OtherActor :type "Actor Object Reference") (OtherComp :type "PrimitiveComponent Object Reference") (OtherBodyIndex :type Integer))
  (if (`KismetArrayLibrary.Array_Contains` (`self.Targets`) OtherActor)
    (`KismetArrayLibrary.Array_RemoveItem` (`self.Targets`) OtherActor)))

(event `/Game/Blueprints/Interfaces/BPI_Tower.OnTowerKill`
  (bind _result (`/Engine/EditorBlueprintResources/StandardMacros.IncrementInt` (`.NumberKills` (break `TowerStats` (`self.TowerStats`))))
    (:`  `
      (bind _structout (setmembers `TowerStats` :`StructRef` (`self.TowerStats`) :`NumberKills` _result))
      (set `self.TowerStats` _structout)
      (`self.UpdateStats`))))

(event `/Game/Blueprints/Interfaces/BPI_Tower.OnTowerDamageDealt`
  (params (InDamageDealt :type "Float (double-precision)"))
  (bind _structout (setmembers `TowerStats` :`StructRef` (`self.TowerStats`) :`DamageDealt` (+ InDamageDealt (`.DamageDealt` (break `TowerStats` (`self.TowerStats`))))))
  (set `self.TowerStats` _structout)
  (`self.UpdateStats`))

(event `/Game/Blueprints/Interfaces/BPI_Tower.OnTowerUpgrade`
  (params (InTowerData :type "TowerData Structure") (InNewIndex :type Integer))
  (bind ((`Attacks` _attacks) (`Range` _range)) (break `TowerData` (`self.TowerData`)))
  (`self.SetTowerData` InTowerData)
  (set `self.TowerUpgradeIndex` InNewIndex)
  (`SphereComponent.SetSphereRadius` (`self.SphereRadius`) _range false)
  (`SceneComponent.SetWorldScale3D` (`self.Decal`) (`KismetMathLibrary.Conv_DoubleToVector` (/ _range 100.0))))

(event `/Game/Blueprints/Interfaces/BPI_Tower.OnDeleteTower`
  (`self.TraceAndUpdatePlot`)
  (`/Engine/EditorBlueprintResources/StandardMacros.IsValid` (`self.SpawnedProjectile`)
    (:`Is Valid`
      (`self.K2_DestroyActor` (`self.SpawnedProjectile`)))
    (:`Is Not Valid`
      _))
  (`self.K2_DestroyActor`))

(event `/Game/Blueprints/Interfaces/BPI_Tower.OnMoveTower`
  (`self.TraceAndUpdatePlot`)
  (set `self.bTowerActive` false))

(fn `FindNextValidTarget`
  (returns (bSuccess :type Boolean) (`AsBP Enemy Base` :type "/Game/Blueprints/Enemy/Units/BP_EnemyBase Object Reference"))
  (bind _output (`|GetArrayItem` (`self.Targets`)))
  (`/Engine/EditorBlueprintResources/StandardMacros.IsValid` _output
    (:`Is Valid`
      (bind _asbp_enemy_base (cast `/Game/Blueprints/Enemy/Units/BP_EnemyBase` _output)
        (:`then`
          (return true _asbp_enemy_base))
        (:`CastFailed`
          (return false null))))
    (:`Is Not Valid`
      (`KismetArrayLibrary.Array_RemoveItem` (`self.Targets`) _output)
      (if (`KismetArrayLibrary.Array_IsEmpty` (`self.Targets`))
        (return false null)
        (else
          (bind (_bsuccess _asbp_enemy_base_2) (`self.FindNextValidTarget`))
          (return _bsuccess _asbp_enemy_base_2))))))

(fn `GetDirectionToEnemy`
  (params (InTarget :type "Actor Object Reference"))
  (returns (ReturnValue :type "Vector Structure"))
  (return (`KismetMathLibrary.MakeVector` (.x (`KismetMathLibrary.Normal` (- (`self.K2_GetActorLocation` InTarget) (`self.K2_GetActorLocation` (`self.SpawnedProjectile`))))) (.y (`KismetMathLibrary.Normal` (- (`self.K2_GetActorLocation` InTarget) (`self.K2_GetActorLocation` (`self.SpawnedProjectile`))))) 1.0)))

(fn `SpawnNewProjectile`
  (bind _returnvalue (`|SpawnActorFromClass` (`self.ProjectileClass`) (`KismetMathLibrary.MakeTransform` (`SceneComponent.K2_GetComponentLocation` (`self.ProjectileSpawn`))) "Undefined" "MultiplyWithRoot" self (`self.TowerData`) null))
  (bind _output_get (set `self.SpawnedProjectile` _returnvalue))
  (`self.K2_AttachToComponent` _output_get (`self.WeaponPropMesh`) "None" "KeepWorld" "KeepRelative" "KeepWorld" false))

(fn `TraceAndUpdatePlot`
  (bind _returnvalue (`self.K2_GetActorLocation`))
  (bind (_outhit _returnvalue_2) (`KismetSystemLibrary.LineTraceSingleForObjects` _returnvalue (- _returnvalue (0.0 0.0 500.0)) (`|MakeArray` "ObjectTypeQuery9" "ObjectTypeQuery1" :!type "EObjectTypeQuery Enum")))
  (if _returnvalue_2
    (bind (_bblockinghit _binitialoverlap _time _distance _location _impactpoint _normal _impactnormal _physmat _hitactor _hitcomponent) (`GameplayStatics.BreakHitResult` _outhit))
    (bind _asbp_tower_plot (cast `/Game/Blueprints/Tower/BP_TowerPlot` _hitactor)
      (:`then`
        (`/Game/Blueprints/Tower/BP_TowerPlot.SlotUpdate` _asbp_tower_plot _hitcomponent false)
        (return))
      (:`CastFailed`
        (return)))
    (else
      (return))))

(fn `UserConstructionScript`)