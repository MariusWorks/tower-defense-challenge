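; BP_TowerPlot is a tower build plot that tracks which of its four box slots are taken.
; BeginPlay registers the four box collisions in a map as free.
; The SlotUpdate event overwrites a given box's taken flag in that map, leaving placement logic to outside callers.
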(event `self.ReceiveBeginPlay`
  (`BlueprintMapLibrary.Map_Add` (`self.BoxMap`) (`self.Box`))
  (`BlueprintMapLibrary.Map_Add` (`self.BoxMap`) (`self.Box1`))
  (`BlueprintMapLibrary.Map_Add` (`self.BoxMap`) (`self.Box2`))
  (`BlueprintMapLibrary.Map_Add` (`self.BoxMap`) (`self.Box3`)))

(event `SlotUpdate`
  (params (InBoxCollision :type "PrimitiveComponent Object Reference") (bPlotTaken :type Boolean))
  (`BlueprintMapLibrary.Map_Add` (`self.BoxMap`) InBoxCollision bPlotTaken))

(fn `UserConstructionScript`)