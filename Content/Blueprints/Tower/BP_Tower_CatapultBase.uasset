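; Catapult tower Blueprint that lobs a preloaded projectile at enemies along a ballistic arc.
; Fire plays an eased timeline swinging the weapon mesh, then finds a valid target, detaches the projectile and launches it with a suggested arc velocity.
; After launch, half the scaled tower cooldown elapses before a new projectile spawns and the arm reverses.
; Clearing IsFiring before that reversal keeps the shared timeline Finished event from launching again.
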(event `self.Fire`
  (`/Engine/EditorBlueprintResources/StandardMacros.IsValid` (`self.SpawnedProjectile`)
    (:`Is Valid`
      (set `self.bIsFiring` true)
      (bind (_direction _newtrack_0) (`Timeline|AnimateCatapult` :!via `PlayFromStart` :!label _label)
        (:`Update`
          (`SceneComponent.K2_SetRelativeRotation` (`self.WeaponPropMesh`) (`KismetMathLibrary.MakeRotator` 0.0 (`|EaseFunction` "ExpoIn" _newtrack_0 10.0 -50.0)) false false))
        (:`Finished`
          (if (`self.bIsFiring`)
            (bind _bsuccess (`self.FindNextValidTarget`))
            (if _bsuccess
              (`self.K2_DetachFromActor` (`self.SpawnedProjectile`) "KeepWorld" "KeepWorld" "KeepWorld")
              (bind _outlaunchvelocity (`GameplayStatics.SuggestProjectileVelocity_CustomArc` (`self.K2_GetActorLocation` (`self.SpawnedProjectile`)) (`self.K2_GetActorLocation` (`|GetArrayItem` (`self.Enemies`) (`self.CurrentEnemyIndex`)))))
              (`/Game/Blueprints/Tower/Projectiles/BP_Projectile_Catapult.Fire` (`self.SpawnedProjectile`) _outlaunchvelocity (`|GetArrayItem` (`self.Enemies`) (`self.CurrentEnemyIndex`)))
              (set `self.SpawnedProjectile` null)
              (`self.QueNewProjectile`))))))))

(event `self.QueNewProjectile`
  (`KismetSystemLibrary.Delay` (/ (* (`self.GetTowerCooldown`) (`self.CooldownMultiplier`)) 2.0))
  (`self.SpawnNewProjectile`)
  (set `self.bIsFiring` false)
  (goto _label :!via `ReverseFromEnd`))

(fn `UserConstructionScript`
  (`parent.UserConstructionScript`))