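; Base tower projectile that homes in on a target and applies the tower's attacks to the enemy it hits.
; Fire sets velocity and a three-second lifespan, then Tick ramps homing acceleration up as the distance to the target shrinks.
; Enemy overlaps apply attacks, spawn BP_Splash at a downward trace hit if splash data exists, and destroy the projectile.
; Other overlaps stop movement and disable further overlaps.
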(event `Fire`
  (params (InVelocity :type "Vector Structure") (InTarget :type "/Game/Blueprints/Enemy/Units/BP_EnemyBase Object Reference"))
  (set `MovementComponent.Velocity` InVelocity (`self.ProjectileMovement`))
  (`/Engine/EditorBlueprintResources/StandardMacros.IsValid` InTarget
    (:`Is Valid`
      (bind _output_get (set `self.Target` InTarget))
      (set `ProjectileMovementComponent.HomingTargetComponent` (`/Game/Blueprints/Enemy/Units/BP_EnemyBase.ProjectileTarget` _output_get) (`self.ProjectileMovement`))
      (set `ProjectileMovementComponent.HomingAccelerationMagnitude` 500.0 (`self.ProjectileMovement`))
      (set `self.InitialLengthToTarget` (`self.GetDistanceToTarget`))
      (`self.SetActorTickEnabled` true))
    (:`Is Not Valid`
      (set `ProjectileMovementComponent.bIsHomingProjectile` false (`self.ProjectileMovement`))))
  (`ActorComponent.Activate` (`self.ProjectileMovement`) false)
  (`self.SetLifeSpan` 3.0))

(event `self.ReceiveTick`
  (params (DeltaSeconds :type "Float (single-precision)"))
  (`/Engine/EditorBlueprintResources/StandardMacros.IsValid` (`self.Target`)
    (:`Is Valid`
      (set `ProjectileMovementComponent.HomingAccelerationMagnitude` (`KismetMathLibrary.Lerp` 50000.0 0.0 (/ (`self.GetDistanceToTarget`) (`self.InitialLengthToTarget`))) (`self.ProjectileMovement`)))))

(event `self.Sphere.OnComponentBeginOverlap`
  (params (OverlappedComponent :type "PrimitiveComponent Object Reference") (OtherActor :type "Actor Object Reference") (OtherComp :type "PrimitiveComponent Object Reference") (OtherBodyIndex :type Integer) (bFromSweep :type Boolean) (SweepResult :type "HitResult Structure (by ref)"))
  (bind _returnvalue (`self.K2_GetActorLocation`))
  (bind ((`SplashRadius` _splashradius) (`SplashAttacks` _splashattacks) (`SplashAttackEffects` _splashattackeffects)) (break `TowerData` (`self.InTowerData`)))
  (bind ((`Attacks` _attacks) (`AttackEffects` _attackeffects)) (break `TowerData` (`self.InTowerData`)))
  (bind ((`SplashAttacks` _splashattacks_2) (`SplashAttackEffects` _splashattackeffects_2)) (break `TowerData` (`self.InTowerData`)))
  (if (`KismetSystemLibrary.DoesImplementInterface` OtherActor "/Game/Blueprints/Interfaces/BPI_Enemy.BPI_Enemy_C")
    (`/Game/Blueprints/Tower/Utility/BPL_Attacks.HandleAttack` self OtherActor (`self.GetOwner`) _attacks _attackeffects)
    (if (or (`KismetArrayLibrary.Array_IsNotEmpty` _splashattacks_2) (`KismetArrayLibrary.Array_IsNotEmpty` _splashattackeffects_2))
      (bind _outhit (`KismetSystemLibrary.LineTraceSingleForObjects` _returnvalue (- _returnvalue (0.0 0.0 500.0)) (`|MakeArray` "ObjectTypeQuery1" "ObjectTypeQuery2" :!type "EObjectTypeQuery Enum") true))
      (`|SpawnActorFromClass` "/Game/Blueprints/Tower/Splash/BP_Splash.BP_Splash_C" (`KismetMathLibrary.MakeTransform` (`.Location` (`GameplayStatics.BreakHitResult` _outhit))) "Undefined" "MultiplyWithRoot" (`self.GetOwner`) _splashradius _splashattacks _splashattackeffects null))
    (`self.K2_DestroyActor`)
    (else
      (`ActorComponent.Deactivate` (`self.ProjectileMovement`))
      (`self.SetActorTickEnabled` false)
      (set `PrimitiveComponent.bGenerateOverlapEvents` false (`self.Sphere`)))))

(fn `GetDistanceToTarget`
  (returns (OutLength :type "Float (double-precision)"))
  (return (`KismetMathLibrary.VSize` (- (`self.K2_GetActorLocation`) (`self.K2_GetActorLocation` (`self.Target`))))))

(fn `UserConstructionScript`)