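; Base tower projectile that delivers attacks and effects to the first enemy it overlaps, identified through BPI_Enemy.
; Attack, effect and splash data come from the tower struct at the current upgrade index.
; On an enemy hit it applies the attack, spawns BP_Splash at a downward trace's hit location if splash data exists, then destroys itself.
; Any other overlap freezes it in place by disabling movement, tick and overlap events.
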(event `self.ReceiveBeginPlay`
  (`/Engine/EditorBlueprintResources/StandardMacros.IsValid` (`self.ProjectileMovement`)
    (:`Is Valid`
      (`KismetSystemLibrary.PrintString` "Projectile Movement Is Valid"))
    (:`Is Not Valid`
      (`KismetSystemLibrary.PrintString` "Projectile Movement Is NOT Valid"))))

(event `self.SphereComponent.OnComponentBeginOverlap`
  (params (OverlappedComponent :type "PrimitiveComponent Object Reference") (OtherActor :type "Actor Object Reference") (OtherComp :type "PrimitiveComponent Object Reference") (OtherBodyIndex :type Integer) (bFromSweep :type Boolean) (SweepResult :type "HitResult Structure (by ref)"))
  (bind (_outsplashattacks _outsplashattackeffects) (`self.GetSplashAttacks`))
  (bind _returnvalue (`self.K2_GetActorLocation`))
  (bind (_outattacks _outattackeffects) (`self.GetAttacks`))
  (if (`KismetSystemLibrary.DoesImplementInterface` OtherActor "/Game/Blueprints/Interfaces/BPI_Enemy.BPI_Enemy_C")
    (`/Game/Blueprints/Tower/Utility/BPL_Attacks.HandleAttack` self OtherActor (`self.GetOwner`) _outattacks _outattackeffects)
    (if (`self.GetHasSplashAttacks`)
      (bind _outhit (`KismetSystemLibrary.LineTraceSingleForObjects` _returnvalue (- _returnvalue (0.0 0.0 500.0)) (`|MakeArray` "ObjectTypeQuery1" "ObjectTypeQuery2" :!type "EObjectTypeQuery Enum") true))
      (`|SpawnActorFromClass` "/Game/Blueprints/Tower/Splash/BP_Splash.BP_Splash_C" (`KismetMathLibrary.MakeTransform` (`.Location` (`GameplayStatics.BreakHitResult` _outhit))) "Undefined" "MultiplyWithRoot" (`self.GetOwner`) 0.0 _outsplashattacks _outsplashattackeffects null))
    (`self.K2_DestroyActor`)
    (else
      (`ActorComponent.Deactivate` (`self.ProjectileMovement`))
      (`self.SetActorTickEnabled` false)
      (set `PrimitiveComponent.bGenerateOverlapEvents` false (`self.SphereComponent`)))))

(fn `GetAttacks`
  (returns (OutAttacks :type "Array of Attack Structure") (OutAttackEffects :type "Array of AttackEffect Structure"))
  (bind (_cost _range _cooldown _splashradius _attacks _attackeffects) (break `TowerData` (`|GetArrayItem` (`.TowerData` (break `TowerStruct` (`self.InTowerStruct`))) (`self.InTowerUpgradeIndex`))))
  (return _attacks _attackeffects))

(fn `GetHasSplashAttacks`
  (returns (bOutHasSplash :type Boolean))
  (bind (_cost _range _cooldown _splashradius _attacks _attackeffects _splashattacks _splashattackeffects) (break `TowerData` (`|GetArrayItem` (`.TowerData` (break `TowerStruct` (`self.InTowerStruct`))) (`self.InTowerUpgradeIndex`))))
  (return (or (`KismetArrayLibrary.Array_IsNotEmpty` _splashattacks) (`KismetArrayLibrary.Array_IsNotEmpty` _splashattackeffects))))

(fn `GetSplashAttacks`
  (returns (OutSplashAttacks :type "Array of Attack Structure") (OutSplashAttackEffects :type "Array of AttackEffect Structure"))
  (bind (_cost _range _cooldown _splashradius _attacks _attackeffects _splashattacks _splashattackeffects) (break `TowerData` (`|GetArrayItem` (`.TowerData` (break `TowerStruct` (`self.InTowerStruct`))) (`self.InTowerUpgradeIndex`))))
  (return _splashattacks _splashattackeffects))

(fn `UserConstructionScript`)