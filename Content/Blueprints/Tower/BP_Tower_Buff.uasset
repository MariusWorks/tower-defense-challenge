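; Support tower Blueprint that buffs the towers in its Targets list rather than showing any attack logic of its own.
; On BeginPlay it sizes the range sphere and hidden decal from TowerData.Range and disables tick.
; Placement and both sphere overlap events reapply a fixed buff through messages to each target; moving or deleting removes it.
; Targets is not populated here, and an unconnected sphere-trace alternative remains in the graph.
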(event `self.ReceiveBeginPlay`
  (bind ((`Range` _range)) (break `TowerData` (`self.TowerData`)))
  (`SphereComponent.SetSphereRadius` (`self.SphereRadius`) _range false)
  (`SceneComponent.SetWorldScale3D` (`self.Decal`) (`KismetMathLibrary.Conv_DoubleToVector` (/ _range 100.0)))
  (`SceneComponent.SetHiddenInGame` (`self.Decal`) true false)
  (`self.SetActorTickEnabled` false))

(event `/Game/Blueprints/Interfaces/BPI_Tower.OnTowerPlaced`
  (`parent.OnTowerPlaced`)
  (for _array_element (`self.Targets`)
    (message `/Game/Blueprints/Interfaces/BPI_Tower.OnApplyBuff` _array_element 0.1)))

(event `/Game/Blueprints/Interfaces/BPI_Tower.OnDeleteTower`
  (for _array_element (`self.Targets`)
    (message `/Game/Blueprints/Interfaces/BPI_Tower.OnRemoveBuff` _array_element))
  (`parent.OnDeleteTower`))

(event `/Game/Blueprints/Interfaces/BPI_Tower.OnMoveTower`
  (for _array_element (`self.Targets`)
    (message `/Game/Blueprints/Interfaces/BPI_Tower.OnRemoveBuff` _array_element))
  (`parent.OnMoveTower`))

(event `self.SphereRadius.OnComponentBeginOverlap`
  (params (OverlappedComponent :type "PrimitiveComponent Object Reference") (OtherActor :type "Actor Object Reference") (OtherComp :type "PrimitiveComponent Object Reference") (OtherBodyIndex :type Integer) (bFromSweep :type Boolean) (SweepResult :type "HitResult Structure (by ref)"))
  (`self.OnTowerPlaced`))

(event `self.SphereRadius.OnComponentEndOverlap`
  (params (OverlappedComponent :type "PrimitiveComponent Object Reference") (OtherActor :type "Actor Object Reference") (OtherComp :type "PrimitiveComponent Object Reference") (OtherBodyIndex :type Integer))
  (`self.OnTowerPlaced`))

(fn `UserConstructionScript`
  (`parent.UserConstructionScript`))