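; Passive support tower that grants buff effects to the towers in its Towers list.
; ChangeBuff applies or removes the PassiveEffects of the current upgrade level, read from TowerStruct, on every tower in that list.
; Placement and any SphereRadius begin-overlap apply the buffs to the whole list, while selling or moving removes them before calling the parent logic.
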(event `TowerInterface.OnTowerPlaced`
  (`self.ChangeBuff` true)
  (`parent.OnTowerPlaced`))

(event `self.SphereRadius.OnComponentBeginOverlap`
  (params (OverlappedComponent :type "PrimitiveComponent Object Reference") (OtherActor :type "Actor Object Reference") (OtherComp :type "PrimitiveComponent Object Reference") (OtherBodyIndex :type Integer) (bFromSweep :type Boolean) (SweepResult :type "HitResult Structure (by ref)"))
  (`self.ChangeBuff` true))

(event `ChangeBuff`
  (params (bApply :type Boolean))
  (for _array_element (`self.Towers`)
    (for _array_element_2 (`.PassiveEffects` (break `TowerData` (`|GetArrayItem` (`.TowerData` (break `TowerStruct` (`self.TowerStruct`))) (`self.GetTowerUpgradeIndex`))))
      (if bApply
        (`TowerInterface.OnTowerApplyBuff` _array_element _array_element_2)
        (else
          (`TowerInterface.OnTowerRemoveBuff` _array_element _array_element_2))))))

(fn `OnTowerMove`
  (returns (ReturnValue :type Boolean))
  (`self.ChangeBuff` false)
  (bind _returnvalue (`parent.OnTowerMove`))
  (return _returnvalue))

(fn `OnTowerSell`
  (returns (ReturnValue :type Boolean))
  (`self.ChangeBuff` false)
  (bind _returnvalue (`parent.OnTowerSell`))
  (return _returnvalue))

(fn `UserConstructionScript`
  (`parent.UserConstructionScript`))