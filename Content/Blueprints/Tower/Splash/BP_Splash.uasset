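; BP_Splash is a tower splash effect actor that damages enemies touching it while its decal fades away.
; On BeginPlay it gives the decal a dynamic material instance, and Tick lerps its Opacity parameter to zero over a fixed fade time, then destroys the actor.
; The sphere's begin-overlap event applies flat damage to BP_EnemyBase actors only, once per overlap entry, regardless of how far the fade has progressed.
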(event `self.ReceiveBeginPlay`
  (bind _returnvalue (`KismetMaterialLibrary.CreateDynamicMaterialInstance` (`DecalComponent.DecalMaterial` (`self.Decal`))))
  (bind _output_get (set `self.DynamicDecalMaterial` _returnvalue))
  (`DecalComponent.SetDecalMaterial` (`self.Decal`) _output_get)
  (set `self.FadeTime` 10.0))

(event `self.ReceiveTick`
  (params (DeltaSeconds :type "Float (single-precision)"))
  (set `self.CurrentTime` (+ DeltaSeconds (`self.CurrentTime`)))
  (`MaterialInstanceDynamic.SetScalarParameterValue` (`self.DynamicDecalMaterial`) "Opacity" (`KismetMathLibrary.Lerp` 1.0 0.0 (`KismetMathLibrary.FClamp` (/ (`self.CurrentTime`) (`self.FadeTime`)))))
  (if (> (`self.CurrentTime`) (`self.FadeTime`))
    (`self.SetActorTickEnabled` false)
    (`self.K2_DestroyActor`)))

(event `self.Sphere.OnComponentBeginOverlap`
  (params (OverlappedComponent :type "PrimitiveComponent Object Reference") (OtherActor :type "Actor Object Reference") (OtherComp :type "PrimitiveComponent Object Reference") (OtherBodyIndex :type Integer) (bFromSweep :type Boolean) (SweepResult :type "HitResult Structure (by ref)"))
  (bind _asbp_enemy_base (cast `/Game/Blueprints/Enemy/BP_EnemyBase` OtherActor))
  (`GameplayStatics.ApplyDamage` _asbp_enemy_base 10.0 null null "/Script/Engine.DamageType"))

(fn `UserConstructionScript`)