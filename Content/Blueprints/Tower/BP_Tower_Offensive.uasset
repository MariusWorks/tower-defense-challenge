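; Offensive tower Blueprint that turns its weapon toward the first enemy in its list and fires projectiles on a cooldown.
; A projectile waits pre-spawned on the weapon, launches at the target on a suggested arc velocity, and its replacement spawns after half the cooldown.
; Passive buffs set cooldown and damage multipliers, keeping the stronger on apply and resetting on removal; damage changes also update the waiting projectile.
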(event `self.ReceiveBeginPlay`
  (set `self.CooldownTimer` (`self.GetTowerCooldown`)))

(event `self.ReceiveTick`
  (params (DeltaSeconds :type "Float (single-precision)"))
  (bind _enemies (`self.Enemies`))
  (bind (_returnvalue_roll _returnvalue_pitch _returnvalue_yaw) (`KismetMathLibrary.BreakRotator` (`SceneComponent.K2_GetComponentRotation` (`self.WeaponPropMesh`))))
  (bind (_returnvalue_roll_2 _returnvalue_pitch_2 _returnvalue_yaw_2) (`KismetMathLibrary.BreakRotator` (`KismetMathLibrary.FindLookAtRotation` (`SceneComponent.K2_GetComponentLocation` (`self.WeaponBaseMesh`)) (`self.K2_GetActorLocation` (`|GetArrayItem` _enemies)))))
  (if (`self.GetTowerActive`)
    (set `self.CooldownTimer` (+ DeltaSeconds (`self.CooldownTimer`)))
    (if (`KismetArrayLibrary.Array_IsNotEmpty` _enemies)
      (`SceneComponent.K2_SetWorldRotation` (`self.WeaponBaseMesh`) (`KismetMathLibrary.MakeRotator` 0.0 0.0 _returnvalue_yaw_2) false false)
      (if (`self.bShouldTowerPitch`)
        (`SceneComponent.K2_SetWorldRotation` (`self.WeaponPropMesh`) (`KismetMathLibrary.MakeRotator` 0.0 _returnvalue_pitch_2 _returnvalue_yaw) false false))
      (if (> (`self.CooldownTimer`) (* (`self.GetTowerCooldown`) (`self.CooldownMultiplier`)))
        (set `self.CooldownTimer` 0.0)
        (bind (_bsuccess _asbp_enemy_base) (`self.FindNextValidTarget`))
        (if _bsuccess
          (set `self.CurrentTarget` _asbp_enemy_base)
          (`self.Fire`))))))

(event `Fire`
  (`/Engine/EditorBlueprintResources/StandardMacros.IsValid` (`self.SpawnedProjectile`)
    (:`Is Valid`
      (`self.K2_DetachFromActor` (`self.SpawnedProjectile`) "KeepWorld" "KeepWorld" "KeepWorld")
      (bind _outlaunchvelocity (`GameplayStatics.SuggestProjectileVelocity_CustomArc` (`self.K2_GetActorLocation` (`self.SpawnedProjectile`)) (`self.K2_GetActorLocation` (`self.CurrentTarget`))))
      (`ProjectileBase.Fire` (`self.SpawnedProjectile`) _outlaunchvelocity (`self.CurrentTarget`))
      (set `self.SpawnedProjectile` null)
      (`self.QueNewProjectile`))))

(event `QueNewProjectile`
  (`KismetSystemLibrary.Delay` (/ (* (`self.GetTowerCooldown`) (`self.CooldownMultiplier`)) 2.0))
  (`self.SpawnNewProjectile`))

(event `TowerInterface.OnTowerApplyBuff`
  (params (InPassiveEffect :type "PassiveEffect Structure"))
  (bind (_passivetype _effectpercent) (break `PassiveEffect` InPassiveEffect))
  (bind _returnvalue (/ _effectpercent 100.0))
  (switch `EPassiveTypes` _passivetype
    (:`CooldownReduction`
      (if (< _returnvalue (`self.CooldownMultiplier`))
        (set `self.CooldownMultiplier` _returnvalue)))
    (:`IncreaseDamage`
      (if (> _returnvalue (`self.DamageMultiplier`))
        (set `self.DamageMultiplier` _returnvalue)
        (`/Engine/EditorBlueprintResources/StandardMacros.IsValid` (`self.SpawnedProjectile`)
          (:`Is Valid`
            (bind _outtowerdata (`self.AddDamageMultiplier`))
            (`ProjectileBase.UpdateProjectileStats` (`self.SpawnedProjectile`) _outtowerdata)))))))

(event `TowerInterface.OnTowerRemoveBuff`
  (params (InPassiveEffect :type "PassiveEffect Structure"))
  (switch `EPassiveTypes` (`.PassiveType` (break `PassiveEffect` InPassiveEffect))
    (:`CooldownReduction`
      (set `self.CooldownMultiplier` 1.0))
    (:`IncreaseDamage`
      (set `self.DamageMultiplier` 1.0)
      (`/Engine/EditorBlueprintResources/StandardMacros.IsValid` (`self.SpawnedProjectile`)
        (:`Is Valid`
          (bind _outtowerdata (`self.AddDamageMultiplier`))
          (`ProjectileBase.UpdateProjectileStats` (`self.SpawnedProjectile`) _outtowerdata))))))

(event `TowerInterface.OnTowerPlaced`
  (`parent.OnTowerPlaced`)
  (`self.SpawnNewProjectile`))

(fn `AddDamageMultiplier`
  (returns (OutTowerData :type "TowerData Structure"))
  (locals (_NewTowerData :type "TowerData Structure"))
  (bind (_towername _towertype _widgetcolor _towerclass _towerdata) (break `TowerStruct` (`self.TowerStruct`)))
  (if (`KismetArrayLibrary.Array_IsNotEmpty` _towerdata)
    (bind _output_get (set `local._NewTowerData` (`|GetArrayItem` _towerdata (`self.GetTowerUpgradeIndex`))))
    (bind (_cost _range _cooldown _splashradius _nexttowertier _attacks _attackeffects _splashattacks) (break `TowerData` _output_get))
    (for (_ _array_index) _attacks
      (bind (_output_damagetype _output_damage) (break `Attack` (`|GetArrayItem` _attacks _array_index)))
      (`|VariableSetRef` _output_damage (* _output_damage (`self.DamageMultiplier`))))
    (for (_ _array_index_2) _splashattacks
      (bind (_output_damagetype_2 _output_damage_2) (break `Attack` (`|GetArrayItem` _splashattacks _array_index_2)))
      (`|VariableSetRef` _output_damage_2 (* _output_damage_2 (`self.DamageMultiplier`))))
    (return (`local._NewTowerData`))))

(fn `FindNextValidTarget`
  (returns (bSuccess :type Boolean) (`AsBP Enemy Base` :type "/Game/Blueprints/Enemy/Units/BP_EnemyBase Object Reference"))
  (bind _output (`|GetArrayItem` (`self.Enemies`)))
  (`/Engine/EditorBlueprintResources/StandardMacros.IsValid` _output
    (:`Is Valid`
      (bind _asbp_enemy_base (cast `/Game/Blueprints/Enemy/Units/BP_EnemyBase` _output)
        (:`then`
          (return true _asbp_enemy_base))
        (:`CastFailed`
          (return false null))))
    (:`Is Not Valid`
      (`KismetArrayLibrary.Array_RemoveItem` (`self.Enemies`) _output)
      (if (`KismetArrayLibrary.Array_IsEmpty` (`self.Enemies`))
        (return false null)
        (else
          (bind (_bsuccess _asbp_enemy_base_2) (`self.FindNextValidTarget`))
          (return _bsuccess _asbp_enemy_base_2))))))

(fn `GetDirectionToEnemy`
  (params (InTarget :type "Actor Object Reference"))
  (returns (ReturnValue :type "Vector Structure"))
  (return (`KismetMathLibrary.MakeVector` (.x (`KismetMathLibrary.Normal` (- (`self.K2_GetActorLocation` InTarget) (`self.K2_GetActorLocation` (`self.SpawnedProjectile`))))) (.y (`KismetMathLibrary.Normal` (- (`self.K2_GetActorLocation` InTarget) (`self.K2_GetActorLocation` (`self.SpawnedProjectile`))))) 1.0)))

(fn `OnRemoveBuff`)

(fn `SpawnNewProjectile`
  (bind _outtowerdata (`self.AddDamageMultiplier`))
  (bind _returnvalue (`|SpawnActorFromClass` (`self.ProjectileClass`) (`KismetMathLibrary.MakeTransform` (`SceneComponent.K2_GetComponentLocation` (`self.ProjectileSpawn`))) "Undefined" "MultiplyWithRoot" self _outtowerdata null))
  (bind _output_get (set `self.SpawnedProjectile` _returnvalue))
  (`self.K2_AttachToComponent` _output_get (`self.WeaponPropMesh`) "None" "KeepWorld" "KeepRelative" "KeepWorld" false))

(fn `UserConstructionScript`
  (`parent.UserConstructionScript`))