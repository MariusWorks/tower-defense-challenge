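; BP_EnemyBase is an enemy actor that travels along a referenced spline and can be damaged.
; Tick advances distance by MovementSpeed, matches the spline's location and rotation, and at the final point notifies BP_PlayerController before destroying the enemy.
; AnyDamage lowers health and updates the health widget.
; The death check subtracts damage again from the reduced health, so the enemy can die with health remaining.
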(event `self.ReceiveBeginPlay`
  (set `self.CurrentHealth` (`self.MaxHealth`))
  (bind _aswbp_enemy_health (cast `/Game/Widget/WBP_EnemyHealth` (`WidgetComponent.GetWidget` (`self.Widget`))))
  (set `self.WidgetEnemyHealthRef` _aswbp_enemy_health))

(event `self.ReceiveAnyDamage`
  (params (Damage :type "Float (single-precision)") (DamageType :type "DamageType Object Reference") (InstigatedBy :type "Controller Object Reference") (DamageCauser :type "Actor Object Reference"))
  (bind _returnvalue (- (`self.CurrentHealth`) Damage))
  (set `self.CurrentHealth` _returnvalue)
  (`/Game/Widget/WBP_EnemyHealth.ChangeHealth` (`self.WidgetEnemyHealthRef`) (`self.CurrentHealth`) (`self.MaxHealth`))
  (if (<= _returnvalue 0.0)
    (`self.K2_DestroyActor`)))

(event `self.ReceiveTick`
  (params (DeltaSeconds :type "Float (single-precision)"))
  (bind _splineref (`self.SplineRef`))
  (bind _splineref_2 (`self.SplineRef`))
  (bind _output_get (set `self.Distance` (+ (* (`self.MovementSpeed`) DeltaSeconds) (`self.Distance`))))
  (`self.K2_SetActorLocation` (`SplineComponent.GetLocationAtDistanceAlongSpline` _splineref _output_get "World"))
  (`self.K2_SetActorRotation` (`SplineComponent.GetRotationAtDistanceAlongSpline` _splineref _output_get "World"))
  (if (>= (`self.Distance`) (`SplineComponent.GetDistanceAlongSplineAtSplinePoint` _splineref_2 (- (`SplineComponent.GetNumberOfSplinePoints` _splineref_2) 1)))
    (bind _asbp_player_controller (cast `/Game/Blueprints/Player/BP_PlayerController` (`GameplayStatics.GetPlayerController` 0)))
    (`/Game/Blueprints/Player/BP_PlayerController.EnemyReachEndEvent` _asbp_player_controller)
    (`self.K2_DestroyActor`)))

(fn `UserConstructionScript`)