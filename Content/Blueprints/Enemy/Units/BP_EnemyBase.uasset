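; Base tower-defense enemy that follows a spline path, notifies the player controller when it reaches the end, and on death awards gold and broadcasts through the game subsystem.
; Tick drives movement plus timed damage-over-time, speed-change and delayed-damage effects, with only the strongest DoT or slow replacing the current one.
; Effect damage routes back through AnyDamage, which updates the health widget and reports damage and kills to the causing tower.
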(event `self.ReceiveBeginPlay`
  (bind ((`CurrentHealth` _currenthealth) (`MaxHealth` _maxhealth)) (break `EnemyData` (`self.EnemyData`)))
  (bind _aswbp_enemy_health (cast `/Game/Widget/WBP_EnemyHealth` (`WidgetComponent.GetWidget` (`self.Widget`))))
  (set `self.WidgetEnemyHealthRef` _aswbp_enemy_health)
  (`/Game/Widget/WBP_EnemyHealth.ChangeHealth` (`self.WidgetEnemyHealthRef`) _currenthealth _maxhealth)
  (set `self.DefaultSpeed` (`.MovementSpeed` (break `EnemyData` (`self.EnemyData`)))))

(event `self.ReceiveAnyDamage`
  (params (Damage :type "Float (single-precision)") (DamageType :type "DamageType Object Reference") (InstigatedBy :type "Controller Object Reference") (DamageCauser :type "Actor Object Reference"))
  (`self.HandleDamage` Damage DamageCauser)
  (if (<= (`.CurrentHealth` (break `EnemyData` (`self.EnemyData`))) 0.0)
    (`/Engine/EditorBlueprintResources/StandardMacros.IsValid` DamageCauser
      (:`Is Valid`
        (message `TowerInterface.OnTowerKill` DamageCauser))
      (:`Is Not Valid`
        _))
    (`GameSubsystem.AddPlayerGold` (subsystem `GameSubsystem`) (`.KillReward` (break `EnemyData` (`self.EnemyData`))))
    (`GameSubsystem.OnEnemyDeath` (subsystem `GameSubsystem`) self)
    (`self.K2_DestroyActor`)))

(event `self.ReceiveTick`
  (params (DeltaSeconds :type "Float (single-precision)"))
  (`self.HandleMovement` DeltaSeconds)
  (if (>= (`self.Distance`) (`SplineComponent.GetDistanceAlongSplineAtSplinePoint` (`self.SplineRef`) (- (`SplineComponent.GetNumberOfSplinePoints` (`self.SplineRef`)) 1)))
    ;[1 0 0] REFACTOR ASAP
    (bind _asbp_player_controller (cast `/Game/Blueprints/Player/BP_PlayerController` (`GameplayStatics.GetPlayerController` 0)))
    (`/Game/Blueprints/Player/BP_PlayerController.EnemyReachEndEvent` _asbp_player_controller)
    (`self.K2_DestroyActor`)
    (else
      (`|ExecutionSequence`
        (:`then_0`
          (if (`self.bHasDamageOverTime`)
            (`self.HandleDamageOverTime` DeltaSeconds)))
        (:`then_1`
          (if (`self.bHasSpeedChange`)
            (`self.HandleSpeedChange` DeltaSeconds)))
        (:`then_2`
          (if (`self.bHasDamagedQueued`)
            (bind _outqueueddamagearray (`self.HandleQueuedDamage` DeltaSeconds))
            (set `self.QueuedDamageArray` _outqueueddamagearray)))))))

(event `/Game/Blueprints/Interfaces/BPI_Enemy.ApplyDamageOverTime`
  (params (InDamageOverTime :type "/Game/Blueprints/Enemy/Utility/S_DamageOverTime Structure"))
  (if (> (`.DamageOverTimeDamage_9_AA5F33714A00077D78C01894370FCB83` (break `/Game/Blueprints/Enemy/Utility/S_DamageOverTime` InDamageOverTime)) (`.DamageOverTimeDamage_9_AA5F33714A00077D78C01894370FCB83` (break `/Game/Blueprints/Enemy/Utility/S_DamageOverTime` (`self.DamagerOverTime`))))
    (set `self.DamagerOverTime` InDamageOverTime)
    (set `self.DamageOverTimeTimer` 0.0)
    (set `self.bHasDamageOverTime` true)))

(event `/Game/Blueprints/Interfaces/BPI_Enemy.ApplySpeedChange`
  (params (InSpeedChange :type "/Game/Blueprints/Enemy/Utility/S_SpeedChange Structure"))
  (if (< (`.SpeedPercent_14_AA5F33714A00077D78C01894370FCB83` (break `/Game/Blueprints/Enemy/Utility/S_SpeedChange` InSpeedChange)) (`.SpeedPercent_14_AA5F33714A00077D78C01894370FCB83` (break `/Game/Blueprints/Enemy/Utility/S_SpeedChange` (`self.SpeedChange`))))
    (bind _output_get (set `self.SpeedChange` InSpeedChange))
    (`|VariableSetRef` (`.MovementSpeed` (break `EnemyData` (`self.EnemyData`))) (* (/ (`.SpeedPercent_14_AA5F33714A00077D78C01894370FCB83` (break `/Game/Blueprints/Enemy/Utility/S_SpeedChange` _output_get)) 100.0) (`.MovementSpeed` (break `EnemyData` (`self.EnemyData`)))))
    (set `self.bHasSpeedChange` true)))

(event `/Game/Blueprints/Interfaces/BPI_Enemy.ApplyQueuedDamage`
  (params (InQueuedDamage :type "/Game/Blueprints/Enemy/Utility/S_QueuedDamage Structure"))
  (set `self.bHasDamagedQueued` true)
  (`KismetArrayLibrary.Array_Add` (`self.QueuedDamageArray`) InQueuedDamage))

(fn `HandleDamage`
  (params (InDamage :type "Float (single-precision)") (InDamageCauser :type "Actor Object Reference"))
  (bind ((`CurrentHealth` _currenthealth)) (break `EnemyData` (`self.EnemyData`)))
  (bind ((`CurrentHealth` _currenthealth_2) (`MaxHealth` _maxhealth)) (break `EnemyData` (`self.EnemyData`)))
  (`|VariableSetRef` _currenthealth (- _currenthealth InDamage))
  (`/Game/Widget/WBP_EnemyHealth.ChangeHealth` (`self.WidgetEnemyHealthRef`) _currenthealth_2 _maxhealth)
  (`/Engine/EditorBlueprintResources/StandardMacros.IsValid` InDamageCauser
    (:`Is Valid`
      (message `TowerInterface.OnTowerDamageDealt` InDamageCauser InDamage))
    (:`Is Not Valid`
      _))
  (return))

(fn `HandleDamageOverTime`
  (params (InDeltaSeconds :type "Float (double-precision)"))
  (bind ((`DamageOverTimeDamage_9_AA5F33714A00077D78C01894370FCB83` _damageovertimedamage) (`DamageOverTimeCauser_10_B8C996D747126F02BC5845986A73665A` _damageovertimecauser)) (break `/Game/Blueprints/Enemy/Utility/S_DamageOverTime` (`self.DamagerOverTime`)))
  (bind ((`DamageDuration_7_1709CEC244EAF83AAB166FA86BBF0DCB` _damageduration)) (break `/Game/Blueprints/Enemy/Utility/S_DamageOverTime` (`self.DamagerOverTime`)))
  (`|VariableSetRef` _damageduration (- _damageduration InDeltaSeconds))
  (if (<= (`.DamageDuration_7_1709CEC244EAF83AAB166FA86BBF0DCB` (break `/Game/Blueprints/Enemy/Utility/S_DamageOverTime` (`self.DamagerOverTime`))) 0.0)
    (set `self.bHasDamageOverTime` false)
    (set `self.DamagerOverTime` (make `/Game/Blueprints/Enemy/Utility/S_DamageOverTime` 0.0 0.0 0.0 null))
    (return)
    (else
      (bind _output_get (set `self.DamageOverTimeTimer` (+ (`local.InDeltaSeconds`) (`self.DamageOverTimeTimer`))))
      (if (> _output_get (`.DamageOverTimeCooldown_8_2372267740775F75333E7791797E37B3` (break `/Game/Blueprints/Enemy/Utility/S_DamageOverTime` (`self.DamagerOverTime`))))
        (set `self.DamageOverTimeTimer` 0.0)
        (`GameplayStatics.ApplyDamage` self _damageovertimedamage null _damageovertimecauser "/Script/Engine.DamageType")))))

(fn `HandleMovement`
  (params (InDeltaSeconds :type "Float (double-precision)"))
  (bind _splineref (`self.SplineRef`))
  (bind _output_get (set `self.Distance` (+ (* InDeltaSeconds (`.MovementSpeed` (break `EnemyData` (`self.EnemyData`)))) (`self.Distance`))))
  (`self.K2_SetActorLocation` (`SplineComponent.GetLocationAtDistanceAlongSpline` _splineref _output_get "World"))
  (`self.K2_SetActorRotation` (`SplineComponent.GetRotationAtDistanceAlongSpline` _splineref _output_get "World"))
  (return))

(fn `HandleQueuedDamage`
  (params (InDeltaSeconds :type "Float (double-precision)"))
  (returns (OutQueuedDamageArray :type "Array of /Game/Blueprints/Enemy/Utility/S_QueuedDamage Structure"))
  (locals (_OutQueuedDamageArray :type "Array of /Game/Blueprints/Enemy/Utility/S_QueuedDamage Structure"))
  (for _array_element (`self.QueuedDamageArray`)
    (bind (_delay _damage _causer) (break `/Game/Blueprints/Enemy/Utility/S_QueuedDamage` _array_element))
    (bind _structout (setmembers `/Game/Blueprints/Enemy/Utility/S_QueuedDamage` :`StructRef` _array_element :`Delay` (- _delay (`local.InDeltaSeconds`))))
    (if (<= _delay 0.0)
      (`GameplayStatics.ApplyDamage` self _damage null _causer "/Script/Engine.DamageType")
      (else
        (`KismetArrayLibrary.Array_Add` (`local._OutQueuedDamageArray`) _structout))))
  (if (`KismetArrayLibrary.Array_IsEmpty` (`local._OutQueuedDamageArray`))
    (set `self.bHasDamagedQueued` false))
  (return (`local._OutQueuedDamageArray`)))

(fn `HandleSpeedChange`
  (params (InDeltaSeconds :type "Float (double-precision)"))
  (bind ((`Duration_12_1709CEC244EAF83AAB166FA86BBF0DCB` _duration)) (break `/Game/Blueprints/Enemy/Utility/S_SpeedChange` (`self.SpeedChange`)))
  (`|VariableSetRef` _duration (- _duration InDeltaSeconds))
  (if (<= (`.Duration_12_1709CEC244EAF83AAB166FA86BBF0DCB` (break `/Game/Blueprints/Enemy/Utility/S_SpeedChange` (`self.SpeedChange`))) 0.0)
    (set `self.bHasSpeedChange` false)
    (set `self.SpeedChange` (make `/Game/Blueprints/Enemy/Utility/S_SpeedChange` 0.0 100.0 null))
    (`|VariableSetRef` (`.MovementSpeed` (break `EnemyData` (`self.EnemyData`))) (`self.DefaultSpeed`))))

(fn `UserConstructionScript`)