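; Enemy wave manager that spawns spline-following enemies at the level's path actor, using a DT_LevelWaves row matched to the level name.
; Player start events enable Tick, which spawns each unit group in turn on its own delay.
; Waves repeat the same cycle with a linearly rising enemy multiplier.
; GameSubsystem events track deaths and announce wave states, with a countdown timer after non-final waves are cleared.
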(event `self.ReceiveBeginPlay`
  (add `GameSubsystem.OnPlayerStartWave` (subsystem `GameSubsystem`) (`|CreateDelegate` :!event `OnPlayerStartWaveEvent`))
  (add `GameSubsystem.OnEnemyDeath` (subsystem `GameSubsystem`) (`|CreateDelegate` :!event `OnEnemyDeathEvent`))
  (bind _returnvalue (`GameplayStatics.GetCurrentLevelName` true))
  (bind _returnvalue_2 (`|GetDataTableRow` "/Game/Data/DT_LevelWaves.DT_LevelWaves" (`KismetStringLibrary.Conv_StringToName` _returnvalue))
    (:`then`
      (set `self.LevelCycle` _returnvalue_2)
      (set `self.CurrentWave` 0)
      (set `self.CurrentWaveUnitsIndex` 0))))

(event `OnPlayerStartWaveEvent`
  (if (`self.bCanStartNewWave`)
    (`KismetSystemLibrary.PrintString` "New Wave Started")
    (if (`KismetSystemLibrary.K2_IsTimerActiveHandle` (`self.NextWaveTimer`))
      (`KismetSystemLibrary.K2_ClearAndInvalidateTimerHandle` (`self.NextWaveTimer`)))
    (set `self.bWaveCompleted` false)
    (set `self.bCanStartNewWave` false)
    (`GameSubsystem.OnWaveStarted` :`self` (subsystem `GameSubsystem`))
    (if (`self.DoesLevelCycleContainEnemies`)
      (set `self.SpawnTimer` (`self.GetUnitSpawnDelay`))
      (`self.SetActorTickEnabled` true))))

(event `self.ReceiveTick`
  (params (DeltaSeconds :type "Float (single-precision)"))
  (bind _pathref (`self.PathRef`))
  (bind _returnvalue (+ (`self.CurrentWave`) 1))
  (bind _returnvalue_2 (+ (`self.CurrentWaveUnitsIndex`) 1))
  (bind _output_get (set `self.SpawnTimer` (+ DeltaSeconds (`self.SpawnTimer`))))
  (if (> _output_get (`self.GetUnitSpawnDelay`))
    (set `self.SpawnTimer` 0.0)
    (bind _asbp_enemy_base (castclass `/Game/Blueprints/Enemy/Units/BP_EnemyBase` (`self.GetUnitClass`)))
    (bind _returnvalue_3 (`|SpawnActorFromClass` _asbp_enemy_base (`KismetMathLibrary.MakeTransform` (`self.K2_GetActorLocation` _pathref)) "Undefined" "MultiplyWithRoot" null (`EnemyPath.SplineComponent` _pathref) (`self.CalculateEnemyMultiplier`) null))
    (`KismetArrayLibrary.Array_Add` (`self.SpawnedEnemies`) _returnvalue_3)
    (bind _result (`/Engine/EditorBlueprintResources/StandardMacros.IncrementInt` (`self.WaveUnitsSpawned`))
      (:`  `
        (if (>= _result (`self.GetUnitsToSpawn`))
          (if (> _returnvalue_2 (`KismetArrayLibrary.Array_LastIndex` (`self.GetCycleUnits`)))
            (set `self.CurrentWaveUnitsIndex` 0)
            (set `self.WaveUnitsSpawned` 0)
            (`self.SetActorTickEnabled` false)
            (set `self.bWaveCompleted` true)
            (if (> _returnvalue (`self.GetLevelCycles`))
              (set `self.bLastWave` true)
              (else
                (set `self.CurrentWave` _returnvalue)
                (set `self.bCanStartNewWave` true)
                (`GameSubsystem.OnNextWaveReady` (subsystem `GameSubsystem`))
                (`KismetSystemLibrary.PrintString` "All Units in wave Spawned, next wave is ready!")))
            (else
              (set `self.CurrentWaveUnitsIndex` _returnvalue_2)
              (set `self.WaveUnitsSpawned` 0))))))))

(event `OnEnemyDeathEvent`
  (params (InEnemyDeath :type "EnemyBase Object Reference"))
  (if (`KismetArrayLibrary.Array_Contains` (`self.SpawnedEnemies`) InEnemyDeath)
    (`KismetArrayLibrary.Array_RemoveItem` (`self.SpawnedEnemies`) InEnemyDeath)
    (if (and (`KismetArrayLibrary.Array_IsEmpty` (`self.SpawnedEnemies`)) (`self.bWaveCompleted`))
      (`GameSubsystem.OnWaveFinished` (subsystem `GameSubsystem`))
      (`KismetSystemLibrary.PrintString` "Wave is finished!")
      (if (`self.bLastWave`)
        (`KismetSystemLibrary.PrintString` "Level Complete")
        (else
          (bind _returnvalue (`KismetSystemLibrary.K2_SetTimerDelegate` (`|CreateDelegate` :!event `OnPlayerStartWaveEvent`) (`self.TimeBetweenWaves`)))
          (set `self.NextWaveTimer` _returnvalue)
          (`GameSubsystem.OnStartWaveCountdownTimer` (subsystem `GameSubsystem`) (`self.TimeBetweenWaves`))
          (`KismetSystemLibrary.PrintString` "Timer Set"))))))

(fn `CalculateEnemyMultiplier`
  (returns (OutEnemyMultiplier :type "Float (double-precision)"))
  (return (+ (* (`self.GetLevelMultiplier`) (`self.CurrentWave`)) 1.0)))

(fn `DoesLevelCycleContainEnemies`
  (returns (ReturnValue :type Boolean))
  (return (`KismetArrayLibrary.Array_IsNotEmpty` (`.CycleUnits` (break `Cycle` (`.Cycle` (break `LevelWaves` (`self.LevelCycle`))))))))

(fn `GetCycleUnits`
  (returns (OutCycleUnits :type "Array of CycleUnit Structure"))
  (return (`.CycleUnits` (break `Cycle` (`.Cycle` (break `LevelWaves` (`self.LevelCycle`)))))))

(fn `GetLevelCycles`
  (returns (OutLevelCycles :type Integer))
  (return (`.LevelCycles` (break `LevelWaves` (`self.LevelCycle`)))))

(fn `GetLevelMultiplier`
  (returns (OutLevelMultiplier :type "Float (double-precision)"))
  (return (`.ScalingMultiplier` (break `LevelWaves` (`self.LevelCycle`)))))

(fn `GetUnitClass`
  (returns (OutUnitClass :type "EnemyBase Class Reference"))
  (return (`.EnemyClass` (break `CycleUnit` (`|GetArrayItem` (`.CycleUnits` (break `Cycle` (`.Cycle` (break `LevelWaves` (`self.LevelCycle`))))) (`self.CurrentWaveUnitsIndex`))))))

(fn `GetUnitSpawnDelay`
  (returns (OutUnitSpawnDelay :type "Float (double-precision)"))
  (return (`.SpawnDelay` (break `CycleUnit` (`|GetArrayItem` (`.CycleUnits` (break `Cycle` (`.Cycle` (break `LevelWaves` (`self.LevelCycle`))))) (`self.CurrentWaveUnitsIndex`))))))

(fn `GetUnitsToSpawn`
  (returns (OutUnitsToSpawn :type Integer))
  (return (`.NumberToSpawn` (break `CycleUnit` (`|GetArrayItem` (`.CycleUnits` (break `Cycle` (`.Cycle` (break `LevelWaves` (`self.LevelCycle`))))) (`self.CurrentWaveUnitsIndex`))))))

(fn `UserConstructionScript`
  (`/Engine/EditorBlueprintResources/StandardMacros.IsValid` (`self.PathRef`)
    (:`Is Not Valid`
      (bind _returnvalue (`GameplayStatics.GetActorOfClass` "/Game/Blueprints/Enemy/BP_EnemyPath.BP_EnemyPath_C"))
      (set `self.PathRef` _returnvalue))))