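; Enemy path actor that builds a spline from an ordered list of tile-like pieces: start, straight, left or right turn, and end.
; ConstructPath resets the heading to the start direction and runs CalculatePathPoints when more than one piece exists.
; GetPathVector maps each piece and current heading to an offset, tangent and new heading, which accumulate into local spline points.
; Tangents are then applied per point to shape the corners.
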(event `ConstructPath`
  (set `self.PathDirection` (`self.StartPathDirection`))
  (if (> (`KismetArrayLibrary.Array_Length` (`self.SplineLocations`)) 1)
    (`self.CalculatePathPoints`)))

(fn `CalculatePathPoints`
  (locals (_CurrentLocation :type "Vector Structure") (NewSplineLocations :type "Array of Vector Structure") (NewTangentArray :type "Array of Vector Structure"))
  (`KismetArrayLibrary.Array_Add` (`local.NewSplineLocations`))
  (for _array_element (`self.SplineLocations`)
    (bind (_outvector _outtangent _outpathdirection) (`self.GetPathVector` _array_element (`self.PathDirection`)))
    (set `self.PathDirection` _outpathdirection)
    (`KismetArrayLibrary.Array_Add` (`local.NewSplineLocations`) (+ _outvector (`local._CurrentLocation`)))
    (`KismetArrayLibrary.Array_Add` (`local.NewTangentArray`) _outtangent)
    (set `local._CurrentLocation` (+ (`local._CurrentLocation`) _outvector)))
  (`SplineComponent.SetSplinePoints` (`self.SplineComponent`) (`local.NewSplineLocations`) "Local" true)
  (for _index (range (`SplineComponent.GetNumberOfSplinePoints` (`self.SplineComponent`)))
    (`SplineComponent.SetTangentAtSplinePoint` (`self.SplineComponent`) _index (`|GetArrayItem` (`local.NewTangentArray`) _index) "Local" true)))

(fn `GetPathVector`
  (params (InPathPiece :type "/Game/Blueprints/Enemy/Utility/E_PathPieces Enum" :default "NewEnumerator0") (InPathDirection :type "/Game/Blueprints/Enemy/Utility/E_PathDirection Enum" :default "NewEnumerator0"))
  (returns (OutVector :type "Vector Structure") (OutTangent :type "Vector Structure") (OutPathDirection :type "/Game/Blueprints/Enemy/Utility/E_PathDirection Enum"))
  (switch `/Game/Blueprints/Enemy/Utility/E_PathPieces` InPathPiece
    (:`NewEnumerator0`
      (switch `/Game/Blueprints/Enemy/Utility/E_PathDirection` (`local.InPathDirection`)
        (:`NewEnumerator0`
          (return (128.5 0.0 0.0) (200.0 0.0 0.0) "NewEnumerator0"))
        (:`NewEnumerator1`
          (return (0.0 128.5 0.0) (0.0 200.0 0.0) "NewEnumerator1"))
        (:`NewEnumerator2`
          (return (-128.5 0.0 0.0) (-200.0 0.0 0.0) "NewEnumerator2"))
        (:`NewEnumerator3`
          (return (0.0 -128.5 0.0) (0.0 -200.0 0.0) "NewEnumerator3"))))
    (:`NewEnumerator1`
      (switch `/Game/Blueprints/Enemy/Utility/E_PathDirection` (`local.InPathDirection`)
        (:`NewEnumerator0`
          (return (260.0 0.0 0.0) (200.0 0.0 0.0) "NewEnumerator0"))
        (:`NewEnumerator1`
          (return (0.0 260.0 0.0) (0.0 200.0 0.0) "NewEnumerator1"))
        (:`NewEnumerator2`
          (return (-260.0 0.0 0.0) (-200.0 0.0 0.0) "NewEnumerator2"))
        (:`NewEnumerator3`
          (return (0.0 -260.0 0.0) (0.0 -200.0 0.0) "NewEnumerator3"))))
    (:`NewEnumerator2`
      (switch `/Game/Blueprints/Enemy/Utility/E_PathDirection` (`local.InPathDirection`)
        (:`NewEnumerator0`
          (return (130.0 130.0 0.0) (200.0 0.0 0.0) "NewEnumerator1"))
        (:`NewEnumerator1`
          (return (-130.0 130.0 0.0) (0.0 200.0 0.0) "NewEnumerator2"))
        (:`NewEnumerator2`
          (return (-130.0 -130.0 0.0) (-200.0 0.0 0.0) "NewEnumerator3"))
        (:`NewEnumerator3`
          (return (130.0 -130.0 0.0) (0.0 -200.0 0.0) "NewEnumerator0"))))
    (:`NewEnumerator3`
      (switch `/Game/Blueprints/Enemy/Utility/E_PathDirection` (`local.InPathDirection`)
        (:`NewEnumerator0`
          (return (130.0 -130.0 0.0) (200.0 0.0 0.0) "NewEnumerator3"))
        (:`NewEnumerator1`
          (return (130.0 130.0 0.0) (0.0 200.0 0.0) "NewEnumerator0"))
        (:`NewEnumerator2`
          (return (-130.0 130.0 0.0) (-200.0 0.0 0.0) "NewEnumerator1"))
        (:`NewEnumerator3`
          (return (-130.0 -130.0 0.0) (0.0 -200.0 0.0) "NewEnumerator2"))))
    (:`NewEnumerator4`
      (switch `/Game/Blueprints/Enemy/Utility/E_PathDirection` (`local.InPathDirection`)
        (:`NewEnumerator0`
          (return (128.5 0.0 0.0) (200.0 0.0 0.0) "NewEnumerator0"))
        (:`NewEnumerator1`
          (return (0.0 128.5 0.0) (0.0 200.0 0.0) "NewEnumerator1"))
        (:`NewEnumerator2`
          (return (-128.5 0.0 0.0) (-200.0 0.0 0.0) "NewEnumerator2"))
        (:`NewEnumerator3`
          (return (0.0 -128.5 0.0) (0.0 -200.0 0.0) "NewEnumerator3"))))))

(fn `UserConstructionScript`)