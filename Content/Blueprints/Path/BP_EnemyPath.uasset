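; BP_EnemyPath is an enemy path actor that spawns BP_EnemyBase enemies along its spline.
; Each Tick it accumulates delta time until the spawn cooldown elapses, then spawns one enemy at the spline's first point in world space.
; It passes its spline reference to each spawned enemy and stops once the spawn count reaches SpawnAmount.
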(event `self.ReceiveTick`
  (params (DeltaSeconds :type "Float (single-precision)"))
  (if (not (>= (`self.SpawnedEnemies`) (`self.SpawnAmount`)))
    (set `self.SpawnCooldownTimer` (+ DeltaSeconds (`self.SpawnCooldownTimer`)))
    (if (> (`self.SpawnCooldownTimer`) (`self.SpawnCooldown`))
      (set `self.SpawnCooldownTimer` 0.0)
      (`|SpawnActorFromClass` "/Game/Blueprints/Enemy/BP_EnemyBase.BP_EnemyBase_C" (`KismetMathLibrary.MakeTransform` (`SplineComponent.GetLocationAtSplinePoint` (`self.Spline`) 0 "World")) "Undefined" "MultiplyWithRoot" null (`self.Spline`) null)
      (`/Engine/EditorBlueprintResources/StandardMacros.IncrementInt` (`self.SpawnedEnemies`)))))

(fn `UserConstructionScript`)